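; BP_VehicleTanksTerra1 is the Terra tank vehicle Blueprint, handling its engine, gear-change and turbo effects.
; Thrust events activate or deactivate high exhaust effects and raise or lower exhaust light intensity, restarting low exhaust on disengage.
; Both gear changes share one burst of side-thrust and backfire effects, while turbo toggles streak and turbo effects.
; GameResetVehicle restores idle low exhaust and dimmer lights; construction just calls the parent.
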(event `self.GameResetVehicle`
  ;[1 1 1] Reset the custom vehicle effects
  (`LightComponent.SetIntensity` (`self.ExhaustLightL2`) 400.0)
  (`LightComponent.SetIntensity` (`self.ExhaustLightR2`) 400.0)
  (`ActorComponent.Deactivate` (`self.EngineThrustSideTR`))
  (`ActorComponent.Deactivate` (`self.EngineThrustSideBR`))
  (`ActorComponent.Deactivate` (`self.EngineThrustSideBL`))
  (`ActorComponent.Deactivate` (`self.EngineThrustSideTL`))
  (`ActorComponent.Deactivate` (`self.TankThrustStreakT`))
  (`ActorComponent.Deactivate` (`self.TankThrustStreakB`))
  (`ActorComponent.Deactivate` (`self.TankThrustStreakL`))
  (`ActorComponent.Deactivate` (`self.TankThrustStreakR`))
  (`ActorComponent.Deactivate` (`self.TankTurboEffect`))
  (`ActorComponent.Deactivate` (`self.EngineExhaustHighR`))
  (`ActorComponent.Deactivate` (`self.EngineExhaustHighT`))
  (`ActorComponent.Deactivate` (`self.EngineExhaustHighB`))
  (`ActorComponent.Deactivate` (`self.EngineExhaustHighL`))
  (`ActorComponent.Activate` (`self.EngineExhaustLowR`) true)
  (`ActorComponent.Activate` (`self.EngineExhaustLowT`) true)
  (`ActorComponent.Activate` (`self.EngineExhaustLowB`) true)
  (`ActorComponent.Activate` (`self.EngineExhaustLowL`) true))

(event `self.ThrustEngaged`
  ;[1 1 1] Thrust engaged
  (`|ExecutionSequence`
    (:`then_0`
      (`ActorComponent.Activate` (`self.EngineExhaustHighR`) false)
      (`ActorComponent.Activate` (`self.EngineExhaustHighT`) false)
      (`ActorComponent.Activate` (`self.EngineExhaustHighB`) false)
      (`ActorComponent.Activate` (`self.EngineExhaustHighL`) false))
    (:`then_1`
      (`LightComponent.SetIntensity` (`self.ExhaustLightL2`) 700.0)
      (`LightComponent.SetIntensity` (`self.ExhaustLightR2`) 700.0))))

(event `self.ThrustDisengaged`
  ;[1 1 1] Thrust disengaged
  (`|ExecutionSequence`
    (:`then_0`
      (`ActorComponent.Deactivate` (`self.EngineExhaustLowB`))
      (`ActorComponent.Deactivate` (`self.EngineExhaustLowT`))
      (`ActorComponent.Deactivate` (`self.EngineExhaustLowR`))
      (`ActorComponent.Deactivate` (`self.EngineExhaustLowL`))
      (`ActorComponent.Activate` (`self.EngineExhaustLowL`) false)
      (`ActorComponent.Activate` (`self.EngineExhaustLowR`) false)
      (`ActorComponent.Activate` (`self.EngineExhaustLowT`) false)
      (`ActorComponent.Activate` (`self.EngineExhaustLowB`) false))
    (:`then_1`
      (`ActorComponent.Deactivate` (`self.EngineExhaustHighR`))
      (`ActorComponent.Deactivate` (`self.EngineExhaustHighT`))
      (`ActorComponent.Deactivate` (`self.EngineExhaustHighB`))
      (`ActorComponent.Deactivate` (`self.EngineExhaustHighL`)))
    (:`then_2`
      (`LightComponent.SetIntensity` (`self.ExhaustLightL2`) 400.0)
      (`LightComponent.SetIntensity` (`self.ExhaustLightR2`) 400.0))))

(event `self.GearUpEngaged`
  ;[1 1 1] Gear change
  (`ActorComponent.Activate` (`self.EngineThrustSideBL`) true :!label _label)
  (`ActorComponent.Activate` (`self.EngineThrustSideTL`) true)
  (`ActorComponent.Activate` (`self.EngineThrustSideTR`) true)
  (`ActorComponent.Activate` (`self.EngineThrustSideBR`) true)
  (`ActorComponent.Activate` (`self.TankBackfireEffectB`) true)
  (`ActorComponent.Activate` (`self.TankBackfireEffectL`) true)
  (`ActorComponent.Activate` (`self.TankBackfireEffectR`) true)
  (`ActorComponent.Activate` (`self.TankBackfireEffectT`) true))

(event `self.GearDownEngaged`
  ;[1 1 1] Gear change
  (goto _label))

(event `self.TurboEngaged`
  ;[1 1 1] Turbo activation
  (`ActorComponent.Activate` (`self.TankThrustStreakT`) false)
  (`ActorComponent.Activate` (`self.TankThrustStreakB`) false)
  (`ActorComponent.Activate` (`self.TankThrustStreakL`) false)
  (`ActorComponent.Activate` (`self.TankThrustStreakR`) false)
  (`ActorComponent.Activate` (`self.TankTurboEffect`) false))

(event `self.TurboDisengaged`
  ;[1 1 1] Turbo activation
  (`ActorComponent.Deactivate` (`self.TankThrustStreakT`))
  (`ActorComponent.Deactivate` (`self.TankThrustStreakB`))
  (`ActorComponent.Deactivate` (`self.TankThrustStreakL`))
  (`ActorComponent.Deactivate` (`self.TankThrustStreakR`))
  (`ActorComponent.Deactivate` (`self.TankTurboEffect`)))

(fn `UserConstructionScript`
  (`parent.UserConstructionScript`))