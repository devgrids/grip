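; Flippable vehicle Blueprint whose graph logic here consists mainly of keyboard debug hacks for play testing.
; Hotkeys kick the cinematics, grant weapon pickups, toggle the AI driver and flip the play game mode's StopWhatYouDoing flag, all blocked in shipping builds.
; The FPS display toggle writes to transient global game state and has no shipping check.
; The construction script is empty and SetShieldExtension is a stub returning false.
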(event `Key|Ctrl+G`
  (params (Key :type "Key Structure"))
  (:`Pressed`
    (bind _returnvalue (`GlobalGameState.IsShippingBuild`))
    (if (not _returnvalue)
      (`self.KickTheCinematics`))))

(event `Key|Three`
  (params (Key :type "Key Structure"))
  (:`Pressed`
    (bind _returnvalue (`GlobalGameState.IsShippingBuild`))
    (if (not _returnvalue)
      (`self.GivePickup` "HomingMissile"))))

(event `Key|Four`
  (params (Key :type "Key Structure"))
  (:`Pressed`
    (bind _returnvalue (`GlobalGameState.IsShippingBuild`))
    (if (not _returnvalue)
      (`self.GivePickup` "GatlingGun"))))

(event `Key|Ctrl+I`
  (params (Key :type "Key Structure"))
  (:`Pressed`
    (bind _returnvalue (`GlobalGameState.IsShippingBuild`))
    (if (not _returnvalue)
      (`self.SetAIDriver` (not (`self.HasAIDriver`))))))

(event `Key|Ctrl+F`
  (params (Key :type "Key Structure"))
  (:`Pressed`
    (bind _returnvalue (`GlobalGameState.GetGlobalGameState` (`GameplayStatics.GetGameInstance`)))
    (bind _transientgamestate (`GlobalGameState.TransientGameState` _returnvalue))
    (setmembers `TransientGameState` :`StructRef` _transientgamestate :`ShowFPS` (not (`.ShowFPS` (break `TransientGameState` _transientgamestate))))))

(event `Key|Ctrl+B`
  (params (Key :type "Key Structure"))
  (:`Pressed`
    (bind _returnvalue (`GlobalGameState.IsShippingBuild`))
    (if (not _returnvalue)
      (bind _asplay_game_mode (cast `PlayGameMode` (`GameplayStatics.GetGameMode`)))
      (set `PlayGameMode.StopWhatYouDoing` (not (`PlayGameMode.StopWhatYouDoing` _asplay_game_mode)) _asplay_game_mode))))

(fn `SetShieldExtension`
  (params (extended :type "Float (double-precision)"))
  (returns (ReturnValue :type Boolean))
  (return false))

(fn `UserConstructionScript`)